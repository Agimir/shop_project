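; Greybox first-person player character with Enhanced Input movement, look and jump, plus a HUD widget created on BeginPlay.
; Interact traces between camera and a point ahead to grab components via PhysicsHandle, releasing on completion; the looping PickedUp hold-position update is never triggered.
; Damage feeds BPComStats, with an M-key self-damage test.
; Sprint and stamina logic is disconnected, and the phone input only delays.
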(event Custom|PickedUp
  (bind _camera (Variables|Default|GetCamera))
  ;[0.15 0.15 0.15 0.5 124] TEST IDEAS
  ;;[0.15 0.15 0.15 0.5 64] Grab / Throw Function
  (Utilities|Time|SetTimerbyEvent (delegate Custom|PickedUp) 0.02 true true)
  (if true
    (Physics|Components|PhysicsHandle|SetTargetLocation (Variables|Default|GetPhysicsHandle) (+ (Transformation|GetWorldLocation _camera) (* (Math|Vector|GetForwardVector (Transformation|GetWorldRotation _camera)) (Variables|Default|GetDistanceLine))))))

(event Custom|UtilizeStamina
  ;[0.15 0.15 0.15 0.5 124] TEST IDEAS
  ;;[0.2706 0.4784 0.281 0.502 34] Player Sprinting Mechanics
  ;;;[0.15 0.15 0.15 0.5] Utilize Stamina
  (Variables|Default|SetCurrentStamina (- (Variables|Default|GetCurrentStamina) 3.0))
  (if (<= (Variables|Default|GetCurrentStamina) 2.0)
    _))

(event Custom|RegenStamina
  ;[0.15 0.15 0.15 0.5 124] TEST IDEAS
  ;;[0.2706 0.4784 0.281 0.502 34] Player Sprinting Mechanics
  ;;;[0.15 0.15 0.15 0.5] Regenerate Stamina
  (Variables|Default|SetCurrentStamina (+ (Variables|Default|GetCurrentStamina) 1.5))
  (if (>= (Variables|Default|GetCurrentStamina) 1e+02)
    (if true
      _)))

(event Input|EnhancedActionEvents|EnhancedInputActionIA_Jump
  (params (ActionValue :type Vector%202D%20Structure) (ElapsedSeconds :type Float%20%28double-precision%29) (TriggeredSeconds :type Float%20%28double-precision%29) (InputAction :type Input%20Action%20Object%20Reference :default "/Game/Greybox/Game/Input/IA_Jump.IA_Jump"))
  ;[0.15 0.15 0.15 0.5 124] TEST IDEAS
  ;;[0.15 0.15 0.15 0.5] Player Jump
  (:Triggered
    (Character|Jump))
  (:Completed
    (Character|StopJumping)))

(event Input|EnhancedActionEvents|EnhancedInputActionIA_Phone
  (params (ActionValue :type Boolean) (ElapsedSeconds :type Float%20%28double-precision%29) (TriggeredSeconds :type Float%20%28double-precision%29) (InputAction :type Input%20Action%20Object%20Reference :default "/Game/Greybox/Game/Input/IA_Phone.IA_Phone"))
  ;[0.15 0.15 0.15 0.5 124] Player Control
  (Utilities|FlowControl|Delay 0.2))

(event Input|EnhancedActionEvents|EnhancedInputActionIA_Interact
  (params (ActionValue :type Vector :default "0, 0, 0") (ElapsedSeconds :type Float%20%28double-precision%29) (TriggeredSeconds :type Float%20%28double-precision%29) (InputAction :type Input%20Action%20Object%20Reference :default "/Game/Greybox/Game/Input/IA_Interact.IA_Interact"))
  ;[0.15 0.15 0.15 0.5 124] TEST IDEAS
  ;;[0.15 0.15 0.15 0.5 64] Grab / Throw Function
  (:Started
    (bind (_start _end) (CallFunction|LineTraceChar-Obj))
    (bind (_outhit _returnvalue) (Collision|LineTraceByChannel _start _end "TraceTypeQuery1" false 0 "None"))
    (if _returnvalue
      (Physics|Components|PhysicsHandle|GrabComponentatLocationwithRotation (Variables|Default|GetPhysicsHandle) (.HitComponent (Collision|BreakHitResult _outhit)) "None" (Transformation|GetWorldLocation (.HitComponent (Collision|BreakHitResult _outhit))) "0, 0, 0")))
  (:Completed
    (if true
      (Physics|Components|PhysicsHandle|ReleaseComponent (Variables|Default|GetPhysicsHandle)))))

(event Input|EnhancedActionEvents|EnhancedInputActionIA_Sprint
  (params (ActionValue :type Vector%202D%20Structure) (ElapsedSeconds :type Float%20%28double-precision%29) (TriggeredSeconds :type Float%20%28double-precision%29) (InputAction :type Input%20Action%20Object%20Reference :default "/Game/Greybox/Game/Input/IA_Sprint.IA_Sprint"))
  ;[0.15 0.15 0.15 0.5 124] TEST IDEAS
  ;;[0.2706 0.4784 0.281 0.502 34] Player Sprinting Mechanics
  ;;;[0.15 0.15 0.15 0.5] Sprint Logic
)

(event Input|EnhancedActionEvents|EnhancedInputActionIA_Movement
  (params (ActionValue :type Vector%202D%20Structure) (ElapsedSeconds :type Float%20%28double-precision%29) (TriggeredSeconds :type Float%20%28double-precision%29) (InputAction :type Input%20Action%20Object%20Reference :default "/Game/Greybox/Game/Input/IA_Movement.IA_Movement"))
  (bind _returnvalue (Pawn|GetControlRotation :!class /Script/Engine.Pawn))
  ;[0.15 0.15 0.15 0.5 124] Player Control
  ;;[0.15 0.15 0.15 0.5] Player Movement Function
  ;;;[0.15 0.15 0.15 0.5] Left / Right Movement
  (Pawn|Input|AddMovementInput (Math|Vector|GetRightVector (Math|Rotator|MakeRotator (.roll _returnvalue) 0.0 (.yaw _returnvalue))) (.x ActionValue) false)
  ;;;[0.15 0.15 0.15 0.5] Forward / Back Movement
  (Pawn|Input|AddMovementInput (Math|Vector|GetForwardVector (Math|Rotator|MakeRotator 0.0 0.0 (.yaw _returnvalue))) (.y ActionValue) false))

(event Input|EnhancedActionEvents|EnhancedInputActionIA_Camera
  (params (ActionValue :type Vector%202D%20Structure) (ElapsedSeconds :type Float%20%28double-precision%29) (TriggeredSeconds :type Float%20%28double-precision%29) (InputAction :type Input%20Action%20Object%20Reference :default "/Game/Greybox/Game/Input/IA_Camera.IA_Camera"))
  ;[0.15 0.15 0.15 0.5 124] Player Control
  ;;[0.15 0.15 0.15 0.5] Player Camera
  (Pawn|Input|AddControllerYawInput (.x ActionValue)) ; Controls up / down movement
  (Pawn|Input|AddControllerPitchInput (.y ActionValue)) ; Controls left / ight movement
)

(event EventBeginPlay
  ;[0.2705 0.4793 0.314 0.502 124] CORE FUNCTIONS
  (Utilities|FlowControl|Sequence
    (:then_0
      ;;[0.15 0.15 0.15 0.5 32] Set Viewport
      (bind _returnvalue (UserInterface|CreateWidget "/Game/Greybox/Game/UI/HUD.HUD_C" (Game|GetPlayerController 0)))
      (bind _output_get (Variables|Default|SetHUD%20Widget _returnvalue))
      (UserInterface|Viewport|AddtoViewport _output_get 0)
      (Variables|/Game/Greybox/Game/UI/HUD.HUD_C|SetPlayer%20Info (Variables|Default|GetHUD%20Widget) self))
    (:then_1
      ;;[0.15 0.15 0.15 0.5 32] Enhanced Input Function
      (bind _asplayer_controller (Utilities|Casting|CastToPlayerController (Pawn|GetController)))
      (Utilities|IsValid (PlayerController|LocalPlayerSubsystems|GetEnhancedInputLocalPlayerSubsystem _asplayer_controller)
        (:Is%20Valid
          (Input|AddMappingContext (PlayerController|LocalPlayerSubsystems|GetEnhancedInputLocalPlayerSubsystem _asplayer_controller) "/Game/Greybox/Game/Input/IMC_Player.IMC_Player" 0 "(bIgnoreAllPressedKeysUntilRelease=True,bForceImmediately=False,bNotifyUserSettings=False)"))))))

(event Game|Damage|EventAnyDamage
  (params (Damage :type Float%20%28single-precision%29) (DamageType :type Damage%20Type%20Object%20Reference) (InstigatedBy :type Controller%20Object%20Reference) (DamageCauser :type Actor%20Object%20Reference))
  ;[0.15 0.15 0.15 0.5 124] TEST IDEAS
  ;;[0.4793 0.455 0.2705 0.502 32] TESTING DAMAGE
  (bind (_zerohealth _remaining_health) (Default|Health-Decrease (Variables|Default|GetBPCom_Stats) Damage))
  (if _zerohealth
    (Development|PrintString (Utilities|String|ToString(Float) _remaining_health))))

(event Input|KeyboardEvents|M
  (params (Key :type Key%20Structure :default "None"))
  ;[0.15 0.15 0.15 0.5 124] TEST IDEAS
  ;;[0.4793 0.455 0.2705 0.502 32] TESTING DAMAGE
  (:Pressed
    (Game|Damage|ApplyDamage self 1e+01 0 0)))

(fn ConstructionScript)

(fn LineTraceChar-Obj
  (bind _camera (Variables|Default|GetCamera))
  (bind _returnvalue (Transformation|GetWorldLocation _camera))
  (return (+ _returnvalue (* (Math|Vector|GetForwardVector (Transformation|GetWorldRotation _camera)) (Variables|Default|GetDistanceLine))) _returnvalue))

(fn Determine|Running
  (Development|PrintString (Utilities|String|ToString(Boolean) (> (Math|Vector|VectorLength (Variables|/Script/Engine.MovementComponent|GetVelocity (Variables|Character|GetCharacterMovement))) 0.0))))