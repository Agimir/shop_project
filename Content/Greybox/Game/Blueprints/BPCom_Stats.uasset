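; Stats component that tracks current and maximum health and stamina for its owner.
; BeginPlay fills both to maximum, and the increase functions add an amount and cap it at the maximum.
; The decrease functions set the value to the incoming amount minus the current value, reversing the commented intent, and return true when the result is zero or below.
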(event EventBeginPlay
  ;[0.15 0.15 0.15 0.5] Set health / stamina at maximum on event start
  (Variables|Health|SetCurrentHealth (Variables|Health|GetMaximumHealth))
  (Variables|Stamina|SetCurrentStamina (Variables|Stamina|GetMaximumStamina)))

(fn Health-Decrease
  (params (Damage :type Float%20%28double-precision%29))
  ;[0.15 0.15 0.15 0.5] Decrease health by "Damage" value
  (Variables|Health|SetCurrentHealth (- Damage (Variables|Health|GetCurrentHealth)))
  ;[0.15 0.15 0.15 0.5] Return value / check for 0 health
  (if (<= (Variables|Health|GetCurrentHealth) 0.0)
    (return true)
    (else
      (return false))))

(fn Health-Increase
  (params (HealingValue :type Float%20%28double-precision%29))
  ;[0.15 0.15 0.15 0.5] Add healing value to health
  (Variables|Health|SetCurrentHealth (+ HealingValue (Variables|Health|GetCurrentHealth)))
  ;[0.15 0.15 0.15 0.5] Set current health to max health if healing > max health
  (if (> (Variables|Health|GetCurrentHealth) (Variables|Health|GetMaximumHealth))
    (Variables|Health|SetCurrentHealth (Variables|Health|GetMaximumHealth))))

(fn Stamina-Decrease
  (params (Energy :type Float%20%28double-precision%29))
  ;[0.15 0.15 0.15 0.5] Decrease stamina by "Energy" value
  (Variables|Stamina|SetCurrentStamina (- Energy (Variables|Stamina|GetCurrentStamina)))
  ;[0.15 0.15 0.15 0.5] Return value / check for 0 stamina
  (if (<= (Variables|Stamina|GetCurrentStamina) 0.0)
    (return true)
    (else
      (return false))))

(fn Stamina-Increase
  (params (Energy :type Float%20%28double-precision%29))
  ;[0.15 0.15 0.15 0.5] Add energy value to stamina
  (Variables|Stamina|SetCurrentStamina (+ Energy (Variables|Stamina|GetCurrentStamina)))
  ;[0.15 0.15 0.15 0.5] Set current stamina to max stamina if energy > max stamina
  (if (> (Variables|Stamina|GetCurrentStamina) (Variables|Stamina|GetMaximumStamina))
    (Variables|Stamina|SetCurrentStamina (Variables|Stamina|GetMaximumStamina))))